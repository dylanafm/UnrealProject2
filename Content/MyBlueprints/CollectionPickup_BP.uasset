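; Collectible pickup actor that adds to the player's pickup count when collected.
; It caches the player's ThirdPersonCharacter at BeginPlay, and any overlap with its trigger updates that count, plays a note sound, spawns an ice impact effect and destroys the actor.
; Two timelines are set up to bob and spin the mesh, but no graph event starts them.
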(event `self.ReceiveBeginPlay`
  (bind _asthird_person_character (cast `/Game/ThirdPersonBP/Blueprints/ThirdPersonCharacter` (`GameplayStatics.GetPlayerCharacter` 0)))
  (set `self.ThePlayer` _asthird_person_character))

(event `self.CollectionTrigger.OnComponentBeginOverlap`
  (params (OverlappedComponent :type "PrimitiveComponent Object Reference") (OtherActor :type "Actor Object Reference") (OtherComp :type "PrimitiveComponent Object Reference") (OtherBodyIndex :type Integer) (bFromSweep :type Boolean) (SweepResult :type "HitResult Structure (by ref)"))
  (bind _returnvalue (`self.K2_GetActorLocation`))
  (`/Game/ThirdPersonBP/Blueprints/ThirdPersonCharacter.UpdatePCount` (`self.ThePlayer`))
  (`GameplayStatics.PlaySoundAtLocation` "/Game/MyAudio/note.note" _returnvalue (struct) 1.0 1.0 0.0 null null null)
  (`GameplayStatics.SpawnEmitterAtLocation` "/Game/InfinityBladeEffects/Effects/FX_Mobile/Impacts/P_Impact_Shield_Ice.P_Impact_Shield_Ice" _returnvalue)
  (`self.K2_DestroyActor`))

(fn `UserConstructionScript`)