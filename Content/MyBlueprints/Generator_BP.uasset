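; Generator actor that the player can fix by pressing F while standing inside its Box trigger.
; It caches the ThirdPersonCharacter on BeginPlay, then uses Box overlaps to show or remove the prompt, toggle its own input and open or close a Gate.
; F passes through that Gate to call GeneratorFix on the character, so the repair logic itself lives outside this Blueprint.
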(event `self.ReceiveBeginPlay`
  (bind _asthird_person_character (cast `/Game/ThirdPersonBP/Blueprints/ThirdPersonCharacter` (`GameplayStatics.GetPlayerCharacter` 0)))
  (set `self.The Player` _asthird_person_character))

(event `Key|F`
  (params (Key :type "Key Structure"))
  (:`Pressed`
    (`/Engine/EditorBlueprintResources/StandardMacros.Gate` true :!label _label
      (:`Exit`
        (`/Game/ThirdPersonBP/Blueprints/ThirdPersonCharacter.GeneratorFix` (`self.The Player`))))))

(event `self.Box.OnComponentBeginOverlap`
  (params (OverlappedComponent :type "PrimitiveComponent Object Reference") (OtherActor :type "Actor Object Reference") (OtherComp :type "PrimitiveComponent Object Reference") (OtherBodyIndex :type Integer) (bFromSweep :type Boolean) (SweepResult :type "HitResult Structure (by ref)"))
  (cast `/Game/ThirdPersonBP/Blueprints/ThirdPersonCharacter` OtherActor)
  (`/Game/ThirdPersonBP/Blueprints/ThirdPersonCharacter.DisplayMessage` (`self.The Player`) "Press F to fix")
  (`self.EnableInput` (`GameplayStatics.GetPlayerController` 0))
  (goto _label :!via `Open`))

(event `self.Box.OnComponentEndOverlap`
  (params (OverlappedComponent :type "PrimitiveComponent Object Reference") (OtherActor :type "Actor Object Reference") (OtherComp :type "PrimitiveComponent Object Reference") (OtherBodyIndex :type Integer))
  (cast `/Game/ThirdPersonBP/Blueprints/ThirdPersonCharacter` OtherActor)
  (`/Game/ThirdPersonBP/Blueprints/ThirdPersonCharacter.RemoveMessage` (`self.The Player`))
  (`self.DisableInput` (`GameplayStatics.GetPlayerController` 0))
  (goto _label :!via `Close`))

(fn `UserConstructionScript`)